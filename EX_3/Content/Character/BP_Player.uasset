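; Player Blueprint with a spring arm, a tintable mesh and E-key interaction with nearby objects.
; The construction script creates a dynamic material on the mesh and feeds the Color variable into its vector parameter.
; BeginPlay aligns the spring arm's yaw and roll to the actor, keeping its pitch.
; Pressing E sends an Interact message to the first overlapping BP_Interactable, without checking that one exists.
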(event `self.ReceiveBeginPlay`
  (bind (_returnvalue_roll _returnvalue_pitch _returnvalue_yaw) (`KismetMathLibrary.BreakRotator` (`self.K2_GetActorRotation`)))
  (bind _springarm (`self.SpringArm`))
  (bind (_relativerotation_roll _relativerotation_pitch) (`KismetMathLibrary.BreakRotator` (`SceneComponent.RelativeRotation` _springarm)))
  (`SceneComponent.K2_SetRelativeRotation` _springarm (`KismetMathLibrary.MakeRotator` _returnvalue_roll _relativerotation_pitch _returnvalue_yaw) false false))

(event `Key|E`
  (params (Key :type "Key Structure"))
  (:`Pressed`
    (message `/Game/FrameWork/BPI_Interact.Interact` (`|GetArrayItem` (`self.GetOverlappingActors` "/Game/FrameWork/BP_Interactable.BP_Interactable_C")))))

(fn `UserConstructionScript`
  (bind _returnvalue (`PrimitiveComponent.CreateDynamicMaterialInstance` (`self.Mesh`) 0 null "None"))
  (`MaterialInstanceDynamic.SetVectorParameterValue` _returnvalue "Param" (`self.Color`)))