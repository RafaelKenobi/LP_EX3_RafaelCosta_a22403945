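; BP_PlayerController is a player controller that moves the controlled pawn and spawns orbs from input.
; MoveForward and MoveRight axes add movement along the control rotation's forward and right vectors, with that rotation copied from the pawn on BeginPlay.
; Releasing the SpawnOrb action spawns a BP_Orb at the pawn's location.
; An unconnected node chain for moving toward the cursor's hit location never runs.
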(event `InputAction|SpawnOrb`
  (params (Key :type "Key Structure"))
  (:`Released`
    (`|SpawnActorFromClass` "/Game/GameElements/BP_Orb.BP_Orb_C" (`KismetMathLibrary.MakeTransform` (`self.K2_GetActorLocation` (`self.K2_GetPawn`))) "Undefined" "MultiplyWithRoot" null null)))

(event `self.ReceiveBeginPlay`
  (`self.SetControlRotation` (`self.K2_GetActorRotation` (`self.K2_GetPawn`))))

(event `self.ReceiveTick`
  (params (DeltaSeconds :type "Float (single-precision)")))

(event `InputAxis|MoveRight`
  (params (AxisValue :type "Float (single-precision)"))
  (`Pawn.AddMovementInput` (`self.K2_GetPawn`) (`KismetMathLibrary.GetRightVector` (`self.GetControlRotation`)) AxisValue false))

(event `InputAxis|MoveForward`
  (params (AxisValue :type "Float (single-precision)"))
  (`Pawn.AddMovementInput` (`self.K2_GetPawn`) (`KismetMathLibrary.GetForwardVector` (`self.GetControlRotation`)) AxisValue false))

(fn `UserConstructionScript`)