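; AI controller for the OtherBot, which runs BT_OtherBot on possession and saves the pawn's start location to the blackboard.
; Perception updates set line of sight, storing the sensed Player-tagged actor and broadcasting PlayerSeen with player pawn 0's location.
; Any other update, including non-player stimuli, clears line of sight.
; Both branches set RemembersPlayer and write player pawn 0's current location as LastSeenLocation.
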(event `self.ReceivePossess`
  (params (PossessedPawn :type "Pawn Object Reference"))
  (`self.RunBehaviorTree` "/Game/AI/BotOther/BT_OtherBot.BT_OtherBot")
  (`BlackboardComponent.SetValueAsVector` (`self.Blackboard`) (`self.OtherBotStartLocaion`) (`self.K2_GetActorLocation` (`self.K2_GetPawn`))))

(event `self.AIPerception.OnTargetPerceptionUpdated`
  (params (Actor :type "Actor Object Reference") (Stimulus :type "AIStimulus Structure"))
  (bind _blackboard (`self.Blackboard`))
  (bind _blackboard_2 (`self.Blackboard`))
  (bind _returnvalue (`self.K2_GetActorLocation` (`GameplayStatics.GetPlayerPawn` 0)))
  (if (and (`self.ActorHasTag` Actor "Player") (`.bSuccessfullySensed` (break `AIStimulus` Stimulus)))
    (`BlackboardComponent.SetValueAsBool` _blackboard_2 (`self.hasLineOfSight?`) true)
    (`BlackboardComponent.SetValueAsObject` _blackboard_2 (`self.Player`) Actor)
    (`BlackboardComponent.SetValueAsVector` _blackboard_2 (`self.lastSeenLocation`) _returnvalue)
    (`BlackboardComponent.SetValueAsBool` _blackboard_2 (`self.RemembersPlayer?`) true)
    (`self.playerSeen` _returnvalue)
    (else
      (`BlackboardComponent.SetValueAsBool` _blackboard (`self.hasLineOfSight?`) false)
      (`BlackboardComponent.SetValueAsVector` _blackboard (`self.lastSeenLocation`) (`self.K2_GetActorLocation` (`GameplayStatics.GetPlayerPawn` 0)))
      (`BlackboardComponent.SetValueAsBool` _blackboard (`self.RemembersPlayer?`) true))))

(fn `UserConstructionScript`)