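; AI controller for a bot that runs BT_BOT and tracks the player through AI perception.
; On possess it stores the start location and binds PlayerSpotted to the player-seen event of BP_OtherBotController instances controlling BP_Bot actors.
; Perception updates line of sight in the blackboard; sightings, losses and shared alerts all record a last seen location and set RemembersPlayer.
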(event `self.ReceivePossess`
  (params (PossessedPawn :type "Pawn Object Reference"))
  (`self.RunBehaviorTree` "/Game/AI/BT_BOT.BT_BOT")
  (`BlackboardComponent.SetValueAsVector` (`self.Blackboard`) (`self.BotStartLocaion`) (`self.K2_GetActorLocation` (`self.K2_GetPawn`)))
  (bind _outactors (`GameplayStatics.GetAllActorsOfClass` "/Game/AI/BP_Bot.BP_Bot_C"))
  (for _array_element _outactors
    (bind _asbp_other_bot_controller (cast `/Game/AI/BotOther/BP_OtherBotController` (`AIBlueprintHelperLibrary.GetAIController` _array_element)))
    (add `/Game/AI/BotOther/BP_OtherBotController.playerSeen` _asbp_other_bot_controller (delegate `PlayerSpotted`))))

(event `PlayerSpotted`
  (params (playerPos :type "Vector Structure"))
  (`self.UpdatePlayerLocation` playerPos))

(event `self.AIPerception.OnTargetPerceptionUpdated`
  (params (Actor :type "Actor Object Reference") (Stimulus :type "AIStimulus Structure"))
  (bind _blackboard (`self.Blackboard`))
  (if (`self.ActorHasTag` Actor "Player")
    (`BlackboardComponent.SetValueAsObject` (`self.Blackboard`) (`self.Player`) Actor)
    (if (`.bSuccessfullySensed` (break `AIStimulus` Stimulus))
      (`BlackboardComponent.SetValueAsBool` (`self.Blackboard`) (`self.hasLineOfSight`) true)
      (`self.UpdatePlayerLocation` (`self.K2_GetActorLocation` (`GameplayStatics.GetPlayerPawn` 0)))
      (else
        (`BlackboardComponent.SetValueAsBool` _blackboard (`self.hasLineOfSight`) false)
        (`BlackboardComponent.SetValueAsVector` _blackboard (`self.lastSeenLocation`) (`self.K2_GetActorLocation` (`GameplayStatics.GetPlayerPawn` 0)))
        (`BlackboardComponent.SetValueAsBool` _blackboard (`self.RemembersPlayer`) true)))))

(fn `UpdatePlayerLocation`
  (params (PlayerPosition :type "Vector Structure"))
  (bind _blackboard (`self.Blackboard`))
  (`BlackboardComponent.SetValueAsVector` _blackboard (`self.lastSeenLocation`) PlayerPosition)
  (`BlackboardComponent.SetValueAsBool` _blackboard (`self.RemembersPlayer`) true)
  (return))

(fn `UserConstructionScript`)